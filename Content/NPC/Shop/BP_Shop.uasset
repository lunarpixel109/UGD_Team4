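; NPC shop Blueprint that transfers items from its inventory to the player's, with no payment step yet.
; Set and clear functions track the player's inventory, wallet and in-shop state; the interact event checks that state but does nothing further.
; BuyItem uses inventory interface messages to remove then add the item, attempting a shop re-add on failure, though that call receives no item.
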(event EventBeginPlay)

(event EventTick
  (params (DeltaSeconds :type Float%20%28single-precision%29)))

(event EventInteractInterface
  (if (Variables|Default|GetPlayerInShop)
    _))

(fn BuyItem
  (params (Item :type D%20Item%20Properties%20Structure))
  (LocalVariables|SetTargetItem Item)
  (bind _success (Class|BPIInventory|RemoveItem(Message) (Variables|Default|GetShopInventory) Item))
  (Variables|Default|SetSuccess _success)
  (if _success
    (bind _success_2 (Class|BPIInventory|AddItem(Message) (Variables|Default|GetPlayerInventory) (LocalVariables|GetTargetItem)))
    (if (not _success_2)
      (bind _success_3 (Class|BPIInventory|AddItem(Message) (Variables|Default|GetShopInventory)))
      (bind _output_get (Variables|Default|SetSuccess _success_3))
      (if _output_get
        _
        (else
          (Utilities|String|LogString "Something Has Went Seriously Wrong")))
      (return (Variables|Default|GetSuccess)))
    (else
      (return (Variables|Default|GetSuccess)))))

(fn SetPlayerReferences
  (params (Inventory :type BPAC%20Inventory%20Component%20Object%20Reference) (Wallet :type BP%20Wallet%20Object%20Reference))
  (Variables|Default|SetPlayerWallet Wallet)
  (Variables|Default|SetPlayerInventory Inventory)
  (Variables|Default|SetPlayerInShop true))

(fn ClearPlayerReferences
  (Variables|Default|SetPlayerWallet 0)
  (Variables|Default|SetPlayerInventory 0)
  (Variables|Default|SetPlayerInShop false))