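; Base actor for world items that the first-person character picks up into the inventory on overlap.
; On BeginPlay it looks up its ItemID in the D_InventoryItemData table and caches the row.
; Sphere overlap calls AddItem on the character's inventory component; on success it refreshes the data, shows a HUD notification and destroys itself.
; The InteractInterface event is present but empty.
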(event OnComponentBeginOverlap(Sphere)
  (params (OverlappedComponent :type Primitive%20Component%20Object%20Reference) (OtherActor :type Actor%20Object%20Reference) (OtherComp :type Primitive%20Component%20Object%20Reference) (OtherBodyIndex :type Integer) (bFromSweep :type Boolean) (SweepResult :type Hit%20Result%20Structure%20%28by%20ref%29))
  (bind _asbp_first_person_character (Utilities|Casting|CastToBP_FirstPersonCharacter OtherActor))
  (bind _success (Default|AddItem (Variables|/Game/FirstPerson/Blueprints/BP_FirstPersonCharacter.BP_FirstPersonCharacter_C|GetBPAC_InventoryComponent _asbp_first_person_character) (Variables|Default|GetItem%20ID) (Variables|Default|GetAmount)))
  (if _success
    (CallFunction|InitialiseItemDataStructure)
    (Default|AddItemNotification (Variables|/Game/FirstPerson/Blueprints/BP_FirstPersonCharacter.BP_FirstPersonCharacter_C|GetPlayerHUD _asbp_first_person_character) (Variables|Default|GetItem%20Data%20Struct) (Variables|Default|GetAmount))
    (Actor|DestroyActor)))

(event EventBeginPlay
  (CallFunction|InitialiseItemDataStructure))

(event Collision|EventActorBeginOverlap
  (params (OtherActor :type Actor%20Object%20Reference)))

(event EventTick
  (params (DeltaSeconds :type Float%20%28single-precision%29)))

(event EventInteractInterface)

(fn ConstructionScript)

(fn InitialiseItemDataStructure
  ;[0.15 0.15 0.15 0.5] Gets table row from data table using its row name and sets it (initialises it)
  (bind _returnvalue (Utilities|GetDataTableRow "/Game/EquipableItems/NewInventory/Data_2/D_InventoryItemData.D_InventoryItemData" (Utilities|String|StringToName (Variables|Default|GetItem%20ID)))
    (:then
      (Variables|Default|SetItem%20Data%20Struct _returnvalue))))