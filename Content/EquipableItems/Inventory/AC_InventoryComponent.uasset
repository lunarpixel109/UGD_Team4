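; Inventory component that holds a ten-slot item array, shown in a W_InventoryBack widget created on BeginPlay.
; The I key toggles the widget, enabling cursor and game-and-UI input on open without restoring them on close.
; PickUpFromLineTrace casts the hit actor to BP_ToolBase, then stacks matching stackable items up to 64 or fills empty slots, looping without a break.
; Each successful write reloads the widget and destroys the actor.
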(event Custom|PickUpFromLineTrace
  (params (HitActor :type Actor%20Object%20Reference))
  (bind _asbp_tool_base (Utilities|Casting|CastToBP_ToolBase HitActor)
    (:then
      (for (_array_element _array_index) (Variables|Default|GetItem)
        (if (Math|Boolean|ANDBoolean (== (.Item_ID (Utilities|Struct|BreakD_ItemProperties _array_element)) (.Item_ID (Utilities|Struct|BreakD_ItemProperties (Variables|/Game/EquipableItems/BP_ToolBase.BP_ToolBase_C|GetItem _asbp_tool_base)))) (.Stackable (Utilities|Struct|BreakD_ItemProperties (Variables|/Game/EquipableItems/BP_ToolBase.BP_ToolBase_C|GetItem _asbp_tool_base))) (<= (+ (.Quantity (Utilities|Struct|BreakD_ItemProperties _array_element)) (.Quantity (Utilities|Struct|BreakD_ItemProperties (Variables|/Game/EquipableItems/BP_ToolBase.BP_ToolBase_C|GetItem _asbp_tool_base)))) 64))
          (Utilities|Array|SetArrayElem (Variables|Default|GetItem) _array_index (Utilities|Struct|MakeD_ItemProperties (.item_id (Variables|/Game/EquipableItems/BP_ToolBase.BP_ToolBase_C|GetItem _asbp_tool_base)) (.type (Variables|/Game/EquipableItems/BP_ToolBase.BP_ToolBase_C|GetItem _asbp_tool_base)) (.displayname (Variables|/Game/EquipableItems/BP_ToolBase.BP_ToolBase_C|GetItem _asbp_tool_base)) "" (+ (.Quantity (Utilities|Struct|BreakD_ItemProperties _array_element)) (.Quantity (Utilities|Struct|BreakD_ItemProperties (Variables|/Game/EquipableItems/BP_ToolBase.BP_ToolBase_C|GetItem _asbp_tool_base)))) (.icon (Variables|/Game/EquipableItems/BP_ToolBase.BP_ToolBase_C|GetItem _asbp_tool_base)) (.value (Variables|/Game/EquipableItems/BP_ToolBase.BP_ToolBase_C|GetItem _asbp_tool_base)) (.pickupmesh (Variables|/Game/EquipableItems/BP_ToolBase.BP_ToolBase_C|GetItem _asbp_tool_base)) (.stackable (Variables|/Game/EquipableItems/BP_ToolBase.BP_ToolBase_C|GetItem _asbp_tool_base)) (.pickupskeletal (Variables|/Game/EquipableItems/BP_ToolBase.BP_ToolBase_C|GetItem _asbp_tool_base))))
          (Default|LoadInventory (Variables|Default|GetInventoryWidget) self :!label _label)
          (Actor|DestroyActor _asbp_tool_base)
          (elif (== (.Quantity (Utilities|Struct|BreakD_ItemProperties _array_element)) 0)
            (Utilities|Array|SetArrayElem (Variables|Default|GetItem) _array_index (Variables|/Game/EquipableItems/BP_ToolBase.BP_ToolBase_C|GetItem _asbp_tool_base))
            (goto _label)))))
    (:CastFailed
      (Development|PrintString "Cast Failed"))))

(event EventBeginPlay
  (bind _returnvalue (Game|GetPlayerController 0))
  ;[0.15 0.15 0.15 0.5] Disaply UI
  (bind _returnvalue_2 (UserInterface|CreateWidget "/Game/EquipableItems/Inventory/UI/W_InventoryBack.W_InventoryBack_C"))
  (Variables|Default|SetInventoryWidget _returnvalue_2)
  (Utilities|Array|Resize (Variables|Default|GetItem) 10)
  (Default|LoadInventory (Variables|Default|GetInventoryWidget) self)
  (Variables|/Script/Engine.PlayerController|SetbShowMouseCursor _returnvalue false)
  (Input|SetInputModeGameOnly _returnvalue false))

(event EventTick
  (params (DeltaSeconds :type Float%20%28single-precision%29)))

(event Input|KeyboardEvents|I
  (params (Key :type Key%20Structure :default "None"))
  (bind _returnvalue (Game|GetPlayerController 0))
  (bind _inventorywidget (Variables|Default|GetInventoryWidget))
  ;[0.15 0.15 0.15 0.5] Disaply UI
  (:Pressed
    (if (Widget|IsVisible (Variables|Default|GetInventoryWidget))
      (Widget|RemovefromParent _inventorywidget)
      (else
        (Variables|/Script/Engine.PlayerController|SetbShowMouseCursor _returnvalue true)
        (Input|SetInputModeGameandUI _returnvalue 0 "DoNotLock" true false)
        (UserInterface|Viewport|AddtoViewport _inventorywidget 0)))))